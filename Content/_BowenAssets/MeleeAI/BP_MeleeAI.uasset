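; BP_MeleeAI is a melee enemy character that punches the player and can be damaged until it is destroyed.
; Overlapping PunchRange plays a hook punch montage and sets IsPunch, during which PunchPlayer overlaps on the player's capsule deal damage.
; TakeDamageMelee tracks clamped health and a percentage, while a widget health bar receives a self reference and turns toward the player each tick.
; SetSpeed adjusts walk speed.
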(event OnComponentBeginOverlap(PunchRange)
  (params (OverlappedComponent :type Primitive%20Component%20Object%20Reference) (OtherActor :type Actor%20Object%20Reference) (OtherComp :type Primitive%20Component%20Object%20Reference) (OtherBodyIndex :type Integer) (bFromSweep :type Boolean) (SweepResult :type Hit%20Result%20Structure%20%28by%20ref%29))
  ;[1 1 1] Attack Player
  (Utilities|Casting|CastToBP_BowenPlayer OtherActor)
  (if (not (Variables|Default|GetIsPunch))
    (Variables|Default|SetIsPunch true)
    (Animation|Montage|PlayMontage (Variables|Character|GetMesh) "/Game/_BowenAssets/MeleeAI/MeleeAI_Hook_Punch_Montage.MeleeAI_Hook_Punch_Montage"
      (:OnCompleted
        (Development|PrintString "Punch Player")
        (Variables|Default|SetIsPunch false)))))

(event OnComponentBeginOverlap(punchPlayer)
  (params (OverlappedComponent :type Primitive%20Component%20Object%20Reference) (OtherActor :type Actor%20Object%20Reference) (OtherComp :type Primitive%20Component%20Object%20Reference) (OtherBodyIndex :type Integer) (bFromSweep :type Boolean) (SweepResult :type Hit%20Result%20Structure%20%28by%20ref%29))
  ;[1 1 1] Attack Player
  (bind _asbp_bowen_player (Utilities|Casting|CastToBP_BowenPlayer OtherActor))
  (if (Math|Conversions|ToBoolean(Integer) (Class|KismetMathLibrary|AndIntInt (Math|Conversions|ToInteger(Boolean) (== (Variables|/Script/Engine.Character|GetCapsuleComponent _asbp_bowen_player) OtherComp)) (Math|Conversions|ToInteger(Boolean) (Variables|Default|GetIsPunch))))
    (Development|PrintString "hit player by melee" true true "(R=1.000000,G=0.037799,B=0.000000,A=1.000000)")
    (Default|PlayerTakeDamage _asbp_bowen_player 1e+01)))

(event EventBeginPlay
  ;[1 1 1] Cast to Player Screen
  (bind _asmelee_aihealth_ui (Utilities|Casting|CastToMeleeAIHealthUI (UserInterface|GetUserWidgetObject (Variables|Default|GetMeleeAIHealthUI))))
  (Variables|/Game/_BowenAssets/UIs/MeleeAIHealthUI.MeleeAIHealthUI_C|SetBP_MeleeAI _asmelee_aihealth_ui self))

(event Collision|EventActorBeginOverlap
  (params (OtherActor :type Actor%20Object%20Reference)))

(event EventTick
  (params (DeltaSeconds :type Float%20%28single-precision%29))
  (bind _meleeaihealthui (Variables|Default|GetMeleeAIHealthUI))
  ;[1 1 1] Health Bar Look Player
  (Transformation|SetWorldRotation _meleeaihealthui (Math|Rotator|FindLookatRotation (Transformation|GetWorldLocation _meleeaihealthui) (Transformation|GetActorLocation (Game|GetPlayerCharacter 0))) false false))

(fn ConstructionScript)

(fn SetSpeed
  (params (Speed :type Float%20%28single-precision%29))
  (Variables|/Script/Engine.CharacterMovementComponent|SetMaxWalkSpeed (Variables|Character|GetCharacterMovement) Speed))

(fn TakeDamageMelee
  (params (DamageMelee :type Float%20%28single-precision%29))
  (bind _output_get (Variables|Default|SetHealthMelee (Math|Float|Clamp(Float) (- (Variables|Default|GetHealthMelee) DamageMelee) 0.0 1e+02)))
  (Variables|Default|SetHealthMeleePercentage (/ _output_get 1e+02))
  (if (<= (Variables|Default|GetHealthMelee) 0.0)
    (Development|PrintString "Melee DIed" true true "(R=1.000000,G=0.061575,B=0.101376,A=1.000000)")
    (Actor|DestroyActor)))
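; BP_Boss is a boss enemy that melee-swipes the player when they come close.
; Overlap with the SwipePlayer trigger plays the swipe montage and holds an IsSwiping flag until it completes, blocking re-triggers.
; While that flag is set, the player's capsule entering SwipeRange deals damage through PlayerTakeDamage, with debug prints on hit and montage completion.
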(event OnComponentBeginOverlap(swipePlayer)
  (params (OverlappedComponent :type Primitive%20Component%20Object%20Reference) (OtherActor :type Actor%20Object%20Reference) (OtherComp :type Primitive%20Component%20Object%20Reference) (OtherBodyIndex :type Integer) (bFromSweep :type Boolean) (SweepResult :type Hit%20Result%20Structure%20%28by%20ref%29))
  (Utilities|Casting|CastToBP_BowenPlayer OtherActor)
  (if (not (Variables|Default|GetisSwiping))
    (Variables|Default|SetisSwiping true)
    (Animation|Montage|PlayMontage (Variables|Character|GetMesh) "/Game/_BowenAssets/MeleeAI/Boss_Swiping_Montage.Boss_Swiping_Montage"
      (:OnCompleted
        (Development|PrintString "Boss hit Player")
        (Variables|Default|SetisSwiping false)))))

(event OnComponentBeginOverlap(swipeRange)
  (params (OverlappedComponent :type Primitive%20Component%20Object%20Reference) (OtherActor :type Actor%20Object%20Reference) (OtherComp :type Primitive%20Component%20Object%20Reference) (OtherBodyIndex :type Integer) (bFromSweep :type Boolean) (SweepResult :type Hit%20Result%20Structure%20%28by%20ref%29))
  (bind _asbp_bowen_player (Utilities|Casting|CastToBP_BowenPlayer OtherActor))
  (if (Math|Conversions|ToBoolean(Integer) (Class|KismetMathLibrary|AndIntInt (Math|Conversions|ToInteger(Boolean) (== (Variables|/Script/Engine.Character|GetCapsuleComponent _asbp_bowen_player) OtherComp)) (Math|Conversions|ToInteger(Boolean) (Variables|Default|GetisSwiping))))
    (Development|PrintString "hit player by Boss" true true "(R=1.000000,G=0.037799,B=0.000000,A=1.000000)")
    (Default|PlayerTakeDamage _asbp_bowen_player 2.0)))

(event EventBeginPlay)

(event Collision|EventActorBeginOverlap
  (params (OtherActor :type Actor%20Object%20Reference)))

(event EventTick
  (params (DeltaSeconds :type Float%20%28single-precision%29)))

(fn ConstructionScript)
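; BP_RangeAI is a ranged enemy that throws projectiles at the player.
; Entering HitRange plays a throw montage, spawning BP_RangeAIProjectile on completion, with a flag blocking overlapping throws.
; While FacePlayer is active, Tick smoothly rotates the actor and turns its health widget toward the player.
; TakeDamage updates health and the percentage, destroying the actor at zero; a separate die event plays the death montage.
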(event OnComponentBeginOverlap(HitRange)
  (params (OverlappedComponent :type Primitive%20Component%20Object%20Reference) (OtherActor :type Actor%20Object%20Reference) (OtherComp :type Primitive%20Component%20Object%20Reference) (OtherBodyIndex :type Integer) (bFromSweep :type Boolean) (SweepResult :type Hit%20Result%20Structure%20%28by%20ref%29))
  ;[0.9044 0.03013 1] Spawn Projectile when enter RangeAI hit zone
  (Utilities|Casting|CastToBP_BowenPlayer OtherActor)
  (if (not (Variables|Default|GetisThrow))
    (Variables|Default|SetisThrow true)
    (Animation|Montage|PlayMontage (Variables|Character|GetMesh) "/Game/_BowenAssets/RangeAI/RangeAI_Throw_Object_Montage.RangeAI_Throw_Object_Montage"
      (:OnCompleted
        (Variables|Default|SetisThrow false)
        (CallFunction|SpawnProj)))))

(event Custom|StopFacePlayer
  ;[0.9307 0.1007 1] Look at Player
  (Variables|Default|SetisFacePlayer false))

(event Custom|FacePlayer
  ;[0.9307 0.1007 1] Look at Player
  (Variables|Default|SetisFacePlayer true))

(event Custom|die
  (if (<= (Variables|Default|GetHealth) 0.0)
    (Animation|Montage|PlayMontage (Variables|Character|GetMesh) "/Game/_BowenAssets/RangeAI/RangeAI_Death_montage.RangeAI_Death_montage")))

(event EventBeginPlay
  ;[1 0 0.07523] cast to Widget
  (bind _asrange_aihealth_ui (Utilities|Casting|CastToRangeAIHealthUI (UserInterface|GetUserWidgetObject (Variables|Default|GetRangeAIHealthUI))))
  (Variables|/Game/_BowenAssets/UIs/RangeAIHealthUI.RangeAIHealthUI_C|SetBP_RnageAI _asrange_aihealth_ui self))

(event Collision|EventActorBeginOverlap
  (params (OtherActor :type Actor%20Object%20Reference)))

(event EventTick
  (params (DeltaSeconds :type Float%20%28single-precision%29))
  (bind _rangeaihealthui (Variables|Default|GetRangeAIHealthUI))
  ;[0.9307 0.1007 1] Look at Player
  (Variables|Default|SetDelta DeltaSeconds)
  (if (Variables|Default|GetisFacePlayer)
    (Transformation|SetActorRotation (Math|Interpolation|RInterpTo (Transformation|GetActorRotation) (Math|Rotator|FindLookatRotation (Transformation|GetActorLocation) (Transformation|GetActorLocation (Game|GetPlayerCharacter 0))) (Variables|Default|GetDelta) 2.0))
    (Transformation|SetWorldRotation _rangeaihealthui (Math|Rotator|FindLookatRotation (Transformation|GetWorldLocation _rangeaihealthui) (Transformation|GetActorLocation (Game|GetPlayerCharacter 0))) false false)))

(fn ConstructionScript)

(fn TakeDamage
  (params (Damage :type Float%20%28single-precision%29))
  (bind _output_get (Variables|Default|SetHealth (Math|Float|Clamp(Float) (- (Variables|Default|GetHealth) Damage) 0.0 1e+02)))
  (Variables|Default|SetHealthPercentage (/ _output_get 1e+02))
  (if (<= (Variables|Default|GetHealth) 0.0)
    (Development|PrintString "Range Died" true true "(R=0.053917,G=0.554426,B=1.000000,A=1.000000)")
    (Actor|DestroyActor)))

(fn SpawnProj
  (Game|SpawnActorfromClass "/Game/_BowenAssets/RangeAI/BP_RangeAIProjectile.BP_RangeAIProjectile_C" (Transformation|GetWorldTransform (Variables|Default|Getspawne%20projectile)) "Undefined" 0 0))